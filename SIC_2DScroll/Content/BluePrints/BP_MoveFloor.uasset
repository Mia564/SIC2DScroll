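; BP_MoveFloor is a floor actor that shuttles back and forth along the world Y axis once the player activates it.
; A hit between its Cube and BP_ThirdPersonCharacter sets IsMove, which nothing in the graph clears.
; BeginPlay records the start Y and a fixed-distance end point.
; Tick applies a MoveY-sized local offset without delta-time scaling or sweep, reversing direction past either bound.
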(event OnComponentHit(cube)
  (params (HitComponent :type Primitive%20Component%20Object%20Reference) (OtherActor :type Actor%20Object%20Reference) (OtherComp :type Primitive%20Component%20Object%20Reference) (NormalImpulse :type Vector :default "0, 0, 0") (Hit :type Hit%20Result%20Structure%20%28by%20ref%29))
  (Utilities|Casting|CastToBP_ThirdPersonCharacter OtherActor)
  (Variables|Default|SetisMove true))

(event EventTick
  (params (DeltaSeconds :type Float%20%28single-precision%29))
  (if (Variables|Default|GetisMove)
    (Transformation|AddActorLocalOffset (Variables|Default|GetMoving%20Location) false false)
    (if (> (.y (Transformation|GetActorLocation)) (Variables|Default|GetEndLocationY))
      (Variables|Default|SetMoving%20Location (Math|Vector|MakeVector 0.0 (* (Variables|Default|GetMoveY) -1.0) 0.0))
      (elif (< (.y (Transformation|GetActorLocation)) (Variables|Default|GetStartLocationY))
        (Variables|Default|SetMoving%20Location (Math|Vector|MakeVector 0.0 (Variables|Default|GetMoveY) 0.0))))))

(event Collision|EventActorBeginOverlap
  (params (OtherActor :type Actor%20Object%20Reference)))

(event EventBeginPlay
  (bind _returnvalue (Transformation|GetActorLocation))
  (Variables|Default|SetEndLocationY (+ (.y _returnvalue) 7.6e+03))
  (Variables|Default|SetStartLocationY (.y _returnvalue))
  (Variables|Default|SetMoving%20Location (Math|Vector|MakeVector 0.0 (Variables|Default|GetMoveY) 0.0)))

(fn ConstructionScript)